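; BP_CPlayerController is a player controller Blueprint that binds number-key shortcuts for menus and saving.
; Keys 2 and 3 toggle the pause menu and level-up UI through the controller's own functions.
; Keys 4 and 5 cast player pawn 0 to CPlayer and call its save and load game data functions.
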(event `Key|Two`
  (params (Key :type "Key Structure"))
  (:`Pressed`
    (`self.TogglePauseMenu`)))

(event `Key|Three`
  (params (Key :type "Key Structure"))
  (:`Pressed`
    (`self.ToggleLevelUpUI`)))

(event `Key|Four`
  (params (Key :type "Key Structure"))
  (:`Pressed`
    (bind _ascplayer (cast `CPlayer` (`GameplayStatics.GetPlayerPawn` 0)))
    (`CPlayer.SaveGameData` _ascplayer)))

(event `Key|Five`
  (params (Key :type "Key Structure"))
  (:`Pressed`
    (bind _ascplayer (cast `CPlayer` (`GameplayStatics.GetPlayerPawn` 0)))
    (`CPlayer.LoadGameData` _ascplayer)))

(fn `UserConstructionScript`)
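; Boss character that hands control to the BT_Boss behavior tree through its AI controller on BeginPlay.
; AttackCBP plays the AttackC section of the bear attack montage.
; ACParticle spawns a batch of scaled-down ATP actors; its random-point box has zero size at the origin, so all target the same spot.
; Sphere trace and radial impulse logic is present but disconnected.
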(event `self.ReceiveBeginPlay`
  (`AIController.RunBehaviorTree` (`AIBlueprintHelperLibrary.GetAIController` self) "/Game/Enemy/BossBear/BT_Boss.BT_Boss"))

(fn `ACParticle`
  (for _ (range 11)
    (bind _returnvalue (`|SpawnActorFromClass` "/Game/Enemy/BossBear/PAT/ATP.ATP_C" (`KismetMathLibrary.Conv_VectorToTransform` (+ (`KismetMathLibrary.RandomPointInBoundingBox` (0.0 0.0 0.0) (`KismetMathLibrary.Conv_DoubleToVector` 0.0)) (0.0 0.0 0.0))) "Undefined" "OverrideRootScale" null null))
    (`self.SetActorRelativeScale3D` _returnvalue (0.1 0.1 0.1))))

(fn `Attack C BP`
  (bind _returnvalue (`SkeletalMeshComponent.GetAnimInstance` (`self.Mesh`)))
  (`AnimInstance.Montage_Play` _returnvalue "/Game/Enemy/BossBear/Montage/Bear_Attack_Montage.Bear_Attack_Montage" 1.0 "MontageLength" 0.0 true)
  (`AnimInstance.Montage_JumpToSection` _returnvalue "AttackC" "/Game/Enemy/BossBear/Montage/Bear_Attack_Montage.Bear_Attack_Montage"))

(fn `UserConstructionScript`)
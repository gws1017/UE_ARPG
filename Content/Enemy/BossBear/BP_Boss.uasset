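; Boss bear enemy Blueprint that starts the BT_Boss behavior tree on its AI controller at BeginPlay.
; AttackCBP plays a named section of the bear attack montage, guarded by an Attacking flag that is never cleared here.
; ACParticle sphere-traces near the world origin and applies mass-scaled radial impulses to static-mesh-rooted actors.
; Player-targeting logic is disconnected, and neither function has a live call in this graph.
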(event `self.ReceiveBeginPlay`
  (`AIController.RunBehaviorTree` (`AIBlueprintHelperLibrary.GetAIController` self) "/Game/Enemy/BossBear/BT_Boss.BT_Boss"))

(event `self.ReceiveTick`
  (params (DeltaSeconds :type "Float (single-precision)")))

(fn `ACParticle`
  (for _ (range 11)
    _)
  (bind _outhits (`KismetSystemLibrary.SphereTraceMultiForObjects` :`End` (+ (0.0 0.0 0.0) (0.0 0.0 10.0)) :`ObjectTypes` (`self.Object Types`) :`DrawDebugType` "ForOneFrame"))
  (for _array_element _outhits
    (bind `_as스태틱_메시_컴포넌트` (cast `StaticMeshComponent` (`Actor.RootComponent` (`.HitActor` (`GameplayStatics.BreakHitResult` _array_element)))))
    (`PrimitiveComponent.AddRadialImpulse` `_as스태틱_메시_컴포넌트` (0.0 0.0 0.0) 1000.0 (* (`PrimitiveComponent.GetMass` `_as스태틱_메시_컴포넌트`) 700.0) "RIF_Linear" false)))

(fn `Attack C BP`
  (params (SectionName :type Name))
  (bind _returnvalue (`SkeletalMeshComponent.GetAnimInstance` (`self.Mesh`)))
  (if (not (`self.bAttacking`))
    (set `self.bAttacking` true)
    (`AnimInstance.Montage_Play` _returnvalue "/Game/Enemy/BossBear/Montage/Bear_Attack_Montage.Bear_Attack_Montage" 1.0 "MontageLength" 0.0 true)
    (`AnimInstance.Montage_JumpToSection` _returnvalue SectionName "/Game/Enemy/BossBear/Montage/Bear_Attack_Montage.Bear_Attack_Montage")))

(fn `UserConstructionScript`)
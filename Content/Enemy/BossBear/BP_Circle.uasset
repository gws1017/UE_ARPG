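; BP_Circle is a short-lived circle indicator in the BossBear enemy folder that animates its area fill and then removes itself.
; On BeginPlay it creates dynamic material instances for the Circum and Area components, using the Circum1Area scalar to set each one's role.
; After a brief delay, a timeline drives the Area material's AreaValue parameter, and the actor destroys itself shortly after the timeline finishes.
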(event `self.ReceiveBeginPlay`
  (`|ExecutionSequence`
    (:`then_0`
      (bind _returnvalue (`DecalComponent.CreateDynamicMaterialInstance` (`self.Circum`)))
      (bind _output_get (set `self.Circum Ref` _returnvalue))
      (`MaterialInstanceDynamic.SetScalarParameterValue` _output_get "Circum1Area" 1.0))
    (:`then_1`
      (bind _returnvalue_2 (`DecalComponent.CreateDynamicMaterialInstance` (`self.Area`)))
      (bind _output_get_2 (set `self.Area Ref` _returnvalue_2))
      (`MaterialInstanceDynamic.SetScalarParameterValue` _output_get_2 "Circum1Area" 0.0))
    (:`then_2`
      (`KismetSystemLibrary.Delay` 0.1)
      (bind (_direction _areavaluealpha) (`Timeline|AreaValueTimeline`)
        (:`Update`
          (`MaterialInstanceDynamic.SetScalarParameterValue` (`self.Area Ref`) "AreaValue" _areavaluealpha))
        (:`Finished`
          (`KismetSystemLibrary.Delay` 0.1)
          (`self.K2_DestroyActor`))))))

(fn `UserConstructionScript`)